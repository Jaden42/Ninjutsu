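; Base character Blueprint for combatants, providing health, melee attacks and death handling.
; On BeginPlay it finds or spawns a shared Character_Manager.
; Attack plays a montage and opens a timed damage window, in which DamageArea damages the first overlapped actor; AttachWeapon snaps the weapon to a mesh socket.
; At zero health it ragdolls, notifies the manager with its controller after a delay, then destroys itself.
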(event `self.ReceiveBeginPlay`
  ;[1 1 1] Character Manager
  (`|ExecutionSequence`
    (:`then_0`
      (bind _outactors (`GameplayStatics.GetAllActorsOfClass` "/Game/Ninjutsu/Blueprints/Character_Manager.Character_Manager_C"))
      (if (== (`KismetArrayLibrary.Array_Length` _outactors) 0)
        (bind _returnvalue (`|SpawnActorFromClass` "/Game/Ninjutsu/Blueprints/Character_Manager.Character_Manager_C" (`KismetMathLibrary.MakeTransform` (0.0 0.0 0.0)) "AdjustIfPossibleButDontSpawnIfColliding" "OverrideRootScale"))
        (set `self.Character Manager` _returnvalue)
        (else
          (set `self.Character Manager` (`KismetArrayLibrary.Array_Get` _outactors)))))))

(event `/Game/Ninjutsu/Blueprints/BlueprintInterface/Health_Damage_Interface.Take Damage`
  (params (Damage :type "Float (single-precision)"))
  ;[1 1 1] Death and Respawn
  (`KismetSystemLibrary.PrintString` "OUCH!!!")
  (bind _output_get (set `self.Health` (- (`self.Health`) Damage)))
  (if (<= _output_get 0.0)
    (`self.DisableInput` null)
    (`PrimitiveComponent.SetSimulatePhysics` (`self.Mesh`) true)
    (`KismetSystemLibrary.Delay` 3.0)
    (bind _ascharacter_manager (cast `/Game/Ninjutsu/Blueprints/Character_Manager` (`self.Character Manager`)))
    (`/Game/Ninjutsu/Blueprints/Character_Manager.Combatant Died` _ascharacter_manager self (`self.GetController`))
    (`self.DetachFromControllerPendingDestroy`)
    (`self.K2_DestroyActor`)
    (`self.EnableInput` null)))

(event `self.Damage Area.OnComponentBeginOverlap`
  (params (OtherActor :type "Actor Object Reference") (OtherComp :type "PrimitiveComponent Object Reference") (OtherBodyIndex :type Integer) (bFromSweep :type Boolean) (SweepResult :type "HitResult Structure (by ref)"))
  ;[1 1 1] Weapon Functionality
  (if (`self.Can Damage`)
    (message `/Game/Ninjutsu/Blueprints/BlueprintInterface/Health_Damage_Interface.Take Damage` OtherActor (`self.Damage`))
    (set `self.Can Damage` false)))

(event `Attack`
  ;[1 1 1] Attack
  (set `self.Can Damage` true)
  (`self.PlayAnimMontage` (`self.Attack Animation`) 1.0 (`self.Attack Animation Montage Start Section`))
  (`KismetSystemLibrary.Delay` 1.0)
  (set `self.Can Damage` false)
  (`self.StopAnimMontage` (`self.Attack Animation`)))

(fn `Attach Weapon`
  (`SceneComponent.K2_AttachTo` (`self.Weapon`) (`self.Mesh`) (`self.WeaponSocket`) "SnapToTargetIncludingScale" true))

(fn `UserConstructionScript`)