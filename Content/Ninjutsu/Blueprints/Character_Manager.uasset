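; Character manager that respawns combatants when they die, for both AI and non-AI controllers.
; CombatantDied spawns a new actor of the dead combatant's class, using randomly selected PlayerStart transforms for location and rotation.
; An AI controller is replaced by a newly spawned one of the same class, while any other controller is reused.
; The resulting controller then possesses the new pawn.
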(event `self.ReceiveBeginPlay`)

(event `self.ReceiveActorBeginOverlap`
  (params (OtherActor :type "Actor Object Reference")))

(event `self.ReceiveTick`
  (params (DeltaSeconds :type "Float (single-precision)")))

(fn `Combatant Died`
  (params (Type :type "Object Object Reference") (Controller :type "Controller Object Reference"))
  (bind _controller (`self.Controller`))
  (set `self.Controller` Controller)
  (bind _outactors (`GameplayStatics.GetAllActorsOfClass` "/Script/Engine.PlayerStart"))
  (bind _asactor (castclass `Actor` (`GameplayStatics.GetObjectClass` Type)))
  (bind _returnvalue (`|SpawnActorFromClass` _asactor (`KismetMathLibrary.MakeTransform` (.location (`self.GetTransform` (`KismetArrayLibrary.Array_Get` _outactors (`KismetMathLibrary.RandomIntegerInRange` 0 (- (`KismetArrayLibrary.Array_Length` _outactors) 1))))) (.rotation (`self.GetTransform` (`KismetArrayLibrary.Array_Get` _outactors (`KismetMathLibrary.RandomIntegerInRange` 0 (- (`KismetArrayLibrary.Array_Length` _outactors) 1)))))) "Undefined" "OverrideRootScale"))
  (bind _aspawn (cast `Pawn` _returnvalue))
  (cast `AIController` _controller
    (:`then`
      (bind _asaicontroller (castclass `AIController` (`GameplayStatics.GetObjectClass` _controller)))
      (bind _returnvalue_2 (`|SpawnActorFromClass` _asaicontroller (`KismetMathLibrary.MakeTransform` (0.0 0.0 0.0)) "Undefined" "OverrideRootScale"))
      (set `self.Controller` _returnvalue_2))
    (:`CastFailed`
      _))
  (`Controller.Possess` (`self.Controller`) _aspawn))

(fn `UserConstructionScript`)